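; BP_Juicer is the visual layer of a juicer station that animates juicing when a juicable item is placed.
; OnJuiceStart tints a new dynamic fluid material with the juice color and shows the fluid mesh.
; A timeline turns the handle and scales the fluid holder vertically.
; On finish it calls the C++ OnJuiceComplete to spawn the item and reset state, then hides the fluid.
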(event `self.OnJuiceStart`
  (params (JuiceColor :type "LinearColor Structure"))
  (bind _returnvalue (`PrimitiveComponent.CreateDynamicMaterialInstance` (`self.FluidMesh`) 0 "/Game/Materials/M_Fluid.M_Fluid" "None")) ; Create A New Dynamic Material
  (`MaterialInstanceDynamic.SetVectorParameterValue` _returnvalue "Color" JuiceColor) ; Apply Color
  (`SceneComponent.SetVisibility` (`self.FluidMesh`) true false) ; Show Fluid Cylinder
  (bind (_direction _wheelturning _fluid_scale) (`Timeline|Timeline` :!via `PlayFromStart`) ; Play Animation Timeline
    (:`Update`
      (`SceneComponent.K2_SetRelativeRotation` (`self.HandleMeshComponent`) (`KismetMathLibrary.MakeRotator` _wheelturning) false false) ; Update Wheel Rotation
      (`SceneComponent.SetRelativeScale3D` (`self.FluidHolder`) (`KismetMathLibrary.MakeVector` 1.0 1.0 _fluid_scale)) ; Update Fluid Scale
    )
    (:`Finished`
      (`self.OnJuiceComplete`) ; Call C++ Function To Spawn Item & Reset Vars
      (`SceneComponent.SetVisibility` (`self.FluidMesh`) false false) ; Hide Fluid Mesh
    )))

(fn `UserConstructionScript`)