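; BP_LevelSettings is a per-level settings Blueprint that strips designated actors from a level in singleplayer games.
; After a short delay on BeginPlay, it casts the game instance to MyGameInstance and checks IsSingleplayer.
; When that flag is set, it destroys every actor in the SingleplayerActorsToDelete array.
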(event `self.ReceiveBeginPlay`
  (`KismetSystemLibrary.Delay` 0.2)
  (bind _asmy_game_instance (cast `MyGameInstance` (`GameplayStatics.GetGameInstance`)))
  (if (`MyGameInstance.bIsSingleplayer` _asmy_game_instance)
    (if (!= (`KismetArrayLibrary.Array_Length` (`self.SingleplayerActorsToDelete`)) 0)
      (for _array_element (`self.SingleplayerActorsToDelete`)
        (`self.K2_DestroyActor` _array_element)))))

(fn `UserConstructionScript`)